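; BP_Grid is a grid actor that lays out a Width by Height field of tiles in its construction script, with no active event logic.
; The Instansed flag selects either lightweight InstancedStaticMesh instances or a separate BP_Tile child actor per cell.
; Both modes space cells by twice the instanced mesh's bounding-box max X, with Height running along X and Width along Y.
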(event EventBeginPlay)

(event Collision|EventActorBeginOverlap
  (params (OtherActor :type Actor%20Object%20Reference)))

(event EventTick
  (params (DeltaSeconds :type Float%20%28single-precision%29)))

(fn ConstructionScript
  (Variables|Default|SetRadius (* (.x (.max (StaticMesh|GetBoundingBox (Variables|/Script/Engine.StaticMeshComponent|GetStaticMesh (Variables|Actor|GetInstancedStaticMesh))))) 2.0))
  (for _index (range 1 (Variables|Default|GetWidth))
    (for _index_2 (range 1 (Variables|Default|GetHeight))
      (if (Variables|Default|GetInstansed?)
        (Components|InstancedStaticMesh|AddInstance (Variables|Actor|GetInstancedStaticMesh) (Math|Transform|MakeTransform (Math|Vector|MakeVector (* (Variables|Default|GetRadius) _index_2) (* (Variables|Default|GetRadius) _index) 0.0)) false)
        (else
          (bind _returnvalue (AddComponent|AddChildActorComponent false (Math|Transform|MakeTransform (Math|Vector|MakeVector (* (Variables|Default|GetRadius) _index_2) (* (Variables|Default|GetRadius) _index) 0.0))))
          (ChildActorComponent|SetChildActorClass _returnvalue "/Game/GridSystem/Grid/BP_Tile.BP_Tile_C"))))))