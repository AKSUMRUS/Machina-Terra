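; BP_Clickable gives its owning actor mouse hover and click feedback, stored under the grid system.
; A custom event binds the owner's click, then caches its static mesh and, if one exists, binds cursor-over events.
; Hovering toggles the mesh's custom depth rendering, as used for highlight effects.
; Each click flips IsClicked and swaps the first material slot between good and bad preview materials.
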(event Custom|OnMouseClicked
  (params (TouchedActor :type Actor%20Object%20Reference) (ButtonPressed :type Key%20Structure :default "None"))
  (bind _staticmeshref (Variables|Default|GetStaticMeshRef))
  (bind _output_get (Variables|Default|SetIsClicked (not (Variables|Default|GetIsClicked))))
  (Utilities|IsValid (Variables|Default|GetStaticMeshRef)
    (:Is%20Valid
      (if _output_get
        (Rendering|Material|SetMaterial _staticmeshref 0 "/Game/GridSystem/Grid/Materials/M_GoodPreview.M_GoodPreview")
        (else
          (Rendering|Material|SetMaterial _staticmeshref 0 "/Game/GridSystem/Grid/Materials/M_BadPreview.M_BadPreview"))))))

(event Custom|OnMouseHoverBegin
  (params (TouchedActor :type Actor%20Object%20Reference))
  (Rendering|SetRenderCustomDepth (Variables|Default|GetStaticMeshRef) true))

(event Custom|OnMouseHoverEnd
  (params (TouchedActor :type Actor%20Object%20Reference))
  (Rendering|SetRenderCustomDepth (Variables|Default|GetStaticMeshRef) false))

(event Custom|CustomEvent
  (bind _returnvalue (Components|GetOwner))
  (bind _returnvalue_2 (Actor|GetComponentbyClass _returnvalue "/Script/Engine.StaticMeshComponent"))
  (EventDispatchers|AssignOnClicked _returnvalue (delegate Custom|OnMouseClicked))
  (Utilities|IsValid _returnvalue_2
    (:Is%20Valid
      (Variables|Default|SetStaticMeshRef _returnvalue_2)
      (EventDispatchers|BindEventtoOnBeginCursorOver _returnvalue (delegate Custom|OnMouseHoverBegin))
      (EventDispatchers|BindEventtoOnEndCursorOver _returnvalue (delegate Custom|OnMouseHoverEnd)))))

(fn ConstructionScript)