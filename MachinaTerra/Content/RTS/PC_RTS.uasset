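; RTS player controller that switches between a View state for selecting and commanding units and a Building state for grid-snapped placement.
; Box traces select BPI_RTS actors (Shift adds, Ctrl grabs matching types), and move orders scatter them over random reachable points.
; The preview's material shows overlap or ore shortage and also gates placement, which deducts ore.
; Edge-scroll camera functions exist, but their call is disconnected.
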(event Custom|Select%20Bots
  (if (Variables|Default|GetShift)
    (Variables|Default|SetHitLocationStart (.Location (CallFunction|GetLocationUnderCursor)) :!label _label)
    (bind _returnvalue (Class|WidgetLayoutLibrary|GetMousePositiononViewport))
    (bind _returnvalue_2 (UserInterface|CreateWidget "/Game/RTS/UMG_Selection.UMG_Selection_C" 0 _returnvalue))
    (bind _output_get (Variables|Default|SetSelectionBox _returnvalue_2))
    (UserInterface|Viewport|AddtoViewport _output_get 0)
    (else
      (bind _arrayelement (Utilities|Array|ReverseforEachLoop (Variables|Default|GetSelectedActors))
        (:LoopBody
          (Class|BPIRTS|DeselectActor(Message) _arrayelement)
          (Utilities|Array|RemoveItem (Variables|Default|GetSelectedActors) _arrayelement))
        (:Completed
          (goto _label))))))

(event Custom|Change%20Overlap%20Material
  (bind _buildingpreview (Variables|Default|GetBuildingPreview))
  (bind _buildingpreview_2 (Variables|Default|GetBuildingPreview))
  (bind _cube (Variables|/Game/GridSystem/Grid/Buildings/BP_Building.BP_Building_C|GetCube _buildingpreview_2))
  ;[1 0.1204 0.3008] Overlap Events
  (if (or (!= (+ (Utilities|Array|Length (Collision|GetOverlappingActors _buildingpreview "/Game/GridSystem/Grid/Tiles/BP_TileMountain.BP_TileMountain_C" :!class /Script/Engine.Actor)) (Utilities|Array|Length (Collision|GetOverlappingActors _buildingpreview "/Game/GridSystem/Grid/Resources/BP_Tree.BP_Tree_C" :!class /Script/Engine.Actor)) (Utilities|Array|Length (Collision|GetOverlappingActors _buildingpreview "/Game/GridSystem/Grid/Buildings/BP_Building.BP_Building_C" :!class /Script/Engine.Actor)) (Utilities|Array|Length (Collision|GetOverlappingActors _buildingpreview "/Game/RTS/AI.AI_C" :!class /Script/Engine.Actor))) 0) (< (Variables|Default|GetOreCount) (Variables|/Game/GridSystem/Grid/Buildings/BP_Building.BP_Building_C|GetCost (Variables|Default|GetBuildingPreview))))
    (Rendering|Material|SetMaterial _cube 0 "/Game/GridSystem/Grid/Materials/M_BadPreview.M_BadPreview")
    (else
      (Rendering|Material|SetMaterial _cube 0 "/Game/GridSystem/Grid/Materials/M_GoodPreview.M_GoodPreview"))))

(event Custom|Finish%20Building
  ;[1 1 1] Building
  (Variables|Default|SetState "NewEnumerator0")
  (Actor|DestroyActor (Variables|Default|GetBuildingPreview))
  (Widget|RemovefromParent (Variables|Default|GetBuildingList))
  (Variables|Default|SetBuildingList 0))

(event Custom|ChangePreviewLocation
  (bind (_hit _location) (CallFunction|GetLocationUnderCursor))
  (bind _locationongrid (CallFunction|GetGridLocation _location))
  ;[1 0.9366 0.08125] Change Preview Location
  (if _hit
    (if (Utilities|Operators|NotEqual(!=) (Transformation|GetWorldLocation (Variables|/Script/Engine.Actor|GetRootComponent (Variables|Default|GetBuildingPreview))) _locationongrid 0.0)
      (Transformation|SetWorldLocation (Variables|/Script/Engine.Actor|GetRootComponent (Variables|Default|GetBuildingPreview)) _locationongrid false false)
      (CallFunction|ChangeOverlapMaterial))))

(event Custom|Start%20Building
  ;[1 1 1] Building
  (Variables|Default|SetState "NewEnumerator1")
  (CallFunction|SpawnPreview)
  (bind _returnvalue (UserInterface|CreateWidget "/Game/GridSystem/Grid/Buildings/UMG_BuildingList.UMG_BuildingList_C"))
  (bind _output_get (Variables|Default|SetBuildingList _returnvalue))
  (UserInterface|Viewport|AddtoViewport _output_get 0))

(event Custom|Spawn%20Preview
  ;[1 1 1] Building
  (bind _returnvalue (Game|SpawnActorfromClass (Variables|Default|GetCurrentBuildingType) (Math|Transform|MakeTransform "0, 0, 0" "0, 0, 0" "1.001000,1.001000,1.001000") "AlwaysSpawn" "MultiplyWithRoot" 0 0))
  (bind _asbp_building (Utilities|Casting|CastToBP_Building _returnvalue))
  (bind _output_get (Variables|Default|SetBuildingPreview _asbp_building))
  (Collision|SetCollisionResponsetoChannel (Variables|/Game/GridSystem/Grid/Buildings/BP_Building.BP_Building_C|GetBoxCollision _output_get) "ECC_Pawn" "ECR_Ignore")
  (CallFunction|ChangeOverlapMaterial))

(event Custom|On%20Object%20Clicked
  (bind _asclickable (Utilities|Casting|CastToBP_Clickable (.hitactor (.HitResult (Class|PlayerController|GetHitResultUnderCursorforObjects (Utilities|Array|MakeArray "ObjectTypeQuery1" "ObjectTypeQuery2") true))))
    (:then
      (Utilities|IsValid (Variables|Default|GetSelectedObject)
        (:Is%20Valid
          (Default|DeselectActor (Variables|Default|GetSelectedObject)))
        (:Is%20Not%20Valid
          _))
      (bind _output_get (Variables|Default|SetSelectedObject _asclickable))
      (Default|SelectActor _output_get))
    (:CastFailed
      (Utilities|IsValid (Variables|Default|GetSelectedObject)
        (:Is%20Valid
          (Default|DeselectActor (Variables|Default|GetSelectedObject))
          (Variables|Default|SetSelectedObject 0))))))

(event Custom|AddOre
  (params (Ore :type Integer))
  (Variables|Default|SetOreCount (+ Ore (Variables|Default|GetOreCount))))

(event Input|EnhancedActionEvents|EnhancedInputActionIA_Select
  (params (ActionValue :type Boolean) (ElapsedSeconds :type Float%20%28double-precision%29) (TriggeredSeconds :type Float%20%28double-precision%29) (InputAction :type Input%20Action%20Object%20Reference :default "/Game/RTS/Inputs/IA_Select.IA_Select"))
  (bind _state (Variables|Default|GetState))
  (:Triggered
    (switch Utilities|FlowControl|Switch|SwitchonE_PlayerState _state
      (:NewEnumerator0
        (CallFunction|DrawBox))))
  (:Started
    (switch Utilities|FlowControl|Switch|SwitchonE_PlayerState _state
      (:NewEnumerator0
        (CallFunction|SelectBots)
        (CallFunction|OnObjectClicked))))
  (:Canceled
    (switch Utilities|FlowControl|Switch|SwitchonE_PlayerState _state :!label _label
      (:NewEnumerator0
        (bind _selectionbox (Variables|Default|GetSelectionBox)
          (:then
            (Widget|RemovefromParent _selectionbox)
            (Variables|Default|SetSelectionBox 0))
          (:else)))
      (:NewEnumerator1
        (CallFunction|PlaceBuilding))))
  (:Completed
    (goto _label)))

(event Input|EnhancedActionEvents|EnhancedInputActionIA_Target
  (params (ActionValue :type Boolean) (ElapsedSeconds :type Float%20%28double-precision%29) (TriggeredSeconds :type Float%20%28double-precision%29) (InputAction :type Input%20Action%20Object%20Reference :default "/Game/RTS/Inputs/IA_Target.IA_Target"))
  (:Started
    (if (Utilities|Array|IsNotEmpty (Variables|Default|GetSelectedActors))
      (CallFunction|MoveActors))))

(event EventTick
  (params (DeltaSeconds :type Float%20%28single-precision%29))
  (switch Utilities|FlowControl|Switch|SwitchonE_PlayerState (Variables|Default|GetState)
    (:NewEnumerator1
      (CallFunction|ChangePreviewLocation))))

(event EventBeginPlay
  (Utilities|FlowControl|DelayUntilNextTick)
  (Utilities|FlowControl|DelayUntilNextTick)
  (Variables|Default|SetViewportSize (Viewport|GetViewportSize))
  (Input|AddMappingContext (PlayerController|LocalPlayerSubsystems|GetEnhancedInputLocalPlayerSubsystem) "/Game/RTS/Inputs/IMC_RTS.IMC_RTS" 0 "(bIgnoreAllPressedKeysUntilRelease=True,bForceImmediately=False,bNotifyUserSettings=False)"))

(event Input|KeyboardEvents|B
  (params (Key :type Key%20Structure :default "None"))
  (:Pressed
    (switch Utilities|FlowControl|Switch|SwitchonE_PlayerState (Variables|Default|GetState)
      (:NewEnumerator0
        (CallFunction|StartBuilding))
      (:NewEnumerator1
        (CallFunction|FinishBuilding)))))

(event Input|KeyboardEvents|LeftCtrl
  (params (Key :type Key%20Structure :default "None"))
  (:Pressed
    (Variables|Default|SetCtrl true))
  (:Released
    (Variables|Default|SetCtrl false)))

(event Input|KeyboardEvents|LeftShift
  (params (Key :type Key%20Structure :default "None"))
  (:Pressed
    (Variables|Default|SetShift true))
  (:Released
    (Variables|Default|SetShift false)))

(fn ConstructionScript)

(fn CanMoveCamera
  (bind _returnvalue (CallFunction|GetScaledMousePosition))
  (bind _viewportsize (Variables|Default|GetViewportSize))
  (bind (_x _y) (Math|Vector2D|BreakVector2D _returnvalue))
  (bind _returnvalue_2 (- _viewportsize _returnvalue))
  (bind (_x_2 _y_2) (Math|Vector2D|BreakVector2D _returnvalue_2))
  (return (Math|Boolean|ANDBoolean (.ReturnValue (Game|Player|GetMousePosition)) (Math|Boolean|ORBoolean (<= _x (Variables|Default|GetMargin)) (<= _y (Variables|Default|GetMargin)) (<= _x_2 (Variables|Default|GetMargin)) (<= _y_2 (Variables|Default|GetMargin))) (not (Input|EnhancedActionValues|GetIA_Select)))))

(fn MoveCamera
  (LocalVariables|SetL-CurrentLocation (CallFunction|GetScaledMousePosition))
  (Utilities|FlowControl|Sequence
    (:then_0
      (if (<= (.x (LocalVariables|GetL-CurrentLocation)) (Variables|Default|GetMargin))
        (LocalVariables|SetL-DirectionX (* (- 1.0 (/ (.x (LocalVariables|GetL-CurrentLocation)) (Variables|Default|GetMargin))) -1.0))
        (elif (<= (- (.x (Variables|Default|GetViewportSize)) (.x (LocalVariables|GetL-CurrentLocation))) (Variables|Default|GetMargin))
          (LocalVariables|SetL-DirectionX (- 1.0 (/ (- (.x (Variables|Default|GetViewportSize)) (.x (LocalVariables|GetL-CurrentLocation))) (Variables|Default|GetMargin))))
          (else
            (LocalVariables|SetL-DirectionX 0.0)))))
    (:then_1
      (if (<= (.y (LocalVariables|GetL-CurrentLocation)) (Variables|Default|GetMargin))
        (LocalVariables|SetL-DirectionY (- 1.0 (/ (.y (LocalVariables|GetL-CurrentLocation)) (Variables|Default|GetMargin))))
        (elif (<= (- (.y (Variables|Default|GetViewportSize)) (.y (LocalVariables|GetL-CurrentLocation))) (Variables|Default|GetMargin))
          (LocalVariables|SetL-DirectionY (* (- 1.0 (/ (- (.y (Variables|Default|GetViewportSize)) (.y (LocalVariables|GetL-CurrentLocation))) (Variables|Default|GetMargin))) -1.0))
          (else
            (LocalVariables|SetL-DirectionY 0.0)))))
    (:then_2
      (Transformation|AddActorWorldOffset (Pawn|GetControlledPawn) (Math|Vector|MakeVector (* (Variables|Default|GetSpeed) (LocalVariables|GetL-DirectionY)) (* (Variables|Default|GetSpeed) (LocalVariables|GetL-DirectionX)) 0.0)))))

(fn GetScaledMousePosition
  (bind _returnvalue (Class|WidgetLayoutLibrary|GetViewportScale))
  (bind _returnvalue_2 (Class|WidgetLayoutLibrary|GetMousePositiononViewport))
  (return (* _returnvalue_2 (Math|Vector2D|MakeVector2D _returnvalue _returnvalue))))

(fn DrawBox
  (LocalVariables|SetL-HitLocation (.Location (CallFunction|GetLocationUnderCursor)))
  (bind _outhits (Class|KismetSystemLibrary|BoxTraceMultiforObjects (+ (/ (+ (Variables|Default|GetHitLocationStart) (LocalVariables|GetL-HitLocation)) 2.0) (Math|Vector|MakeVector 0.0 0.0 (Math|Float|Clamp(Float) (.Z (Math|Vector|BreakVector (/ (- (Variables|Default|GetHitLocationStart) (LocalVariables|GetL-HitLocation)) 2.0))) 1e+02 (.Z (Math|Vector|BreakVector (/ (- (Variables|Default|GetHitLocationStart) (LocalVariables|GetL-HitLocation)) 2.0)))))) (- (+ (/ (+ (Variables|Default|GetHitLocationStart) (LocalVariables|GetL-HitLocation)) 2.0) (Math|Vector|MakeVector 0.0 0.0 (Math|Float|Clamp(Float) (.Z (Math|Vector|BreakVector (/ (- (Variables|Default|GetHitLocationStart) (LocalVariables|GetL-HitLocation)) 2.0))) 1e+02 (.Z (Math|Vector|BreakVector (/ (- (Variables|Default|GetHitLocationStart) (LocalVariables|GetL-HitLocation)) 2.0)))))) "0.000000,0.000000,1.000000") (Math|Vector|VectorGetAbs (Math|Vector|MakeVector (.X (Math|Vector|BreakVector (/ (- (Variables|Default|GetHitLocationStart) (LocalVariables|GetL-HitLocation)) 2.0))) (.Y (Math|Vector|BreakVector (/ (- (Variables|Default|GetHitLocationStart) (LocalVariables|GetL-HitLocation)) 2.0))) (Math|Float|Clamp(Float) (.Z (Math|Vector|BreakVector (/ (- (Variables|Default|GetHitLocationStart) (LocalVariables|GetL-HitLocation)) 2.0))) 1e+02 (.Z (Math|Vector|BreakVector (/ (- (Variables|Default|GetHitLocationStart) (LocalVariables|GetL-HitLocation)) 2.0)))))) "0, 0, 0" (Utilities|Array|MakeArray "ObjectTypeQuery3") false 0 "None" true))
  (CallFunction|HandleMultiHit _outhits))

(fn GetLocationUnderCursor
  (bind _array (Utilities|Array|MakeArray "ObjectTypeQuery1"))
  (bind _hitresult (Class|PlayerController|GetHitResultUnderCursorforObjects _array true))
  (bind (_bblockinghit _binitialoverlap _time _distance _location) (Collision|BreakHitResult _hitresult))
  (return _bblockinghit _location))

(fn HandleMultiHit
  (params (InputPin :type Array%20of%20Hit%20Result%20Structures))
  (for _array_element InputPin
    (if (Utilities|DoesObjectImplementInterface (.HitActor (Collision|BreakHitResult _array_element)) "/Game/RTS/BPI_RTS.BPI_RTS_C")
      (Class|BPIRTS|SelectActor(Message) (.HitActor (Collision|BreakHitResult _array_element)))
      (Utilities|Array|AddUnique (Variables|Default|GetSelectedActors) (.HitActor (Collision|BreakHitResult _array_element)))
      (if (Variables|Default|GetCtrl)
        (bind _returnvalue (Class|BPIRTS|ReturnType(Message) (.HitActor (Collision|BreakHitResult _array_element))))
        (LocalVariables|SetL-Filter _returnvalue)
        (bind _outactors (Actor|GetAllActorswithInterface "/Game/RTS/BPI_RTS.BPI_RTS_C"))
        (for _array_element_2 _outactors
          (bind _returnvalue_2 (Class|BPIRTS|ReturnType(Message) _array_element_2))
          (if (Utilities|Enum|Equal(Enum) _returnvalue_2 (LocalVariables|GetL-Filter))
            (Class|BPIRTS|SelectActor(Message) _array_element_2)
            (Utilities|Array|AddUnique (Variables|Default|GetSelectedActors) _array_element_2)))
        (return)))))

(fn MoveActors
  (LocalVariables|SetL-HitLocation (.Location (CallFunction|GetLocationUnderCursor)))
  (Utilities|Array|Add (LocalVariables|GetL-MoveTo) (LocalVariables|GetL-HitLocation))
  (LocalVariables|SetL-ActorsToMove (Utilities|Array|Length (Variables|Default|GetSelectedActors)))
  (while (and (< (Utilities|Array|Length (LocalVariables|GetL-MoveTo)) (LocalVariables|GetL-ActorsToMove)) (< (LocalVariables|GetL-Increment) 99))
    (Math|Integer|IncrementInt (LocalVariables|GetL-Increment)
      (:%20%20
        (LocalVariables|SetL-TestLocation (.RandomLocation (AI|Navigation|GetRandomReachablePointinRadius (LocalVariables|GetL-HitLocation) 4e+02 0 0)))
        (LocalVariables|SetL-Fail false)
        (bind _array_element (Utilities|Array|ForEachLoopwithBreak (LocalVariables|GetL-MoveTo) :!label _label)
          (:LoopBody
            (if (< (Math|Vector|Distance(Vector) _array_element (LocalVariables|GetL-TestLocation)) 1e+02)
              (LocalVariables|SetL-Fail true)
              (goto _label Break)))
          (:Completed
            (if (not (LocalVariables|GetL-Fail))
              (Utilities|Array|Add (LocalVariables|GetL-MoveTo) (LocalVariables|GetL-TestLocation))))))))
  (for (_array_element_2 _array_index) (Variables|Default|GetSelectedActors)
    (Class|BPIRTS|MoveActor(Message) _array_element_2 (Utilities|Array|Get(acopy) (LocalVariables|GetL-MoveTo) (Math|Integer|Clamp(Integer) _array_index 0 (LocalVariables|GetL-ActorsToMove))))))

(fn PlaceBuilding
  (bind _buildingpreview (Variables|Default|GetBuildingPreview))
  (if (== (Rendering|Material|GetMaterial (Variables|/Game/GridSystem/Grid/Buildings/BP_Building.BP_Building_C|GetCube (Variables|Default|GetBuildingPreview)) 0) "/Game/GridSystem/Grid/Materials/M_GoodPreview.M_GoodPreview")
    (Game|SpawnActorfromClass (Utilities|GetClass _buildingpreview) (Math|Transform|MakeTransform (Transformation|GetWorldLocation (Variables|/Game/GridSystem/Grid/Buildings/BP_Building.BP_Building_C|GetCube _buildingpreview)) "0, 0, 0" "1.000000,1.000000,1.000000") "AlwaysSpawn" "MultiplyWithRoot" 0 0)
    (Variables|Default|SetOreCount (- (Variables|Default|GetOreCount) (Variables|/Game/GridSystem/Grid/Buildings/BP_Building.BP_Building_C|GetCost (Variables|Default|GetBuildingPreview))))
    (CallFunction|FinishBuilding)))

(fn GetGridLocation
  (params (CursorLocation :type Vector))
  (bind _gridoffset (LocalVariables|GetGridOffset))
  (bind _gridsize (LocalVariables|GetGridSize))
  (bind _gridsize_2 (LocalVariables|GetGridSize))
  (bind _gridsize_3 (LocalVariables|GetGridSize))
  (bind _returnvalue (/ _gridsize 2.0))
  (bind _returnvalue_2 (/ _gridsize_3 2.0))
  (return (+ (Math|Vector|MakeVector (+ (* (Math|Conversions|ToFloat(Integer) (Math|Float|Round (/ (- (- (.x CursorLocation) _returnvalue) (.x _gridoffset)) _gridsize_2))) _gridsize_3) _returnvalue_2) (+ (* (Math|Conversions|ToFloat(Integer) (Math|Float|Round (/ (- (- (.y CursorLocation) _returnvalue) (.y _gridoffset)) _gridsize_2))) _gridsize_3) _returnvalue_2) 0.0) (LocalVariables|GetGridOffset))))